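; OneshotEvent is a block actor that awards a point when the third-person character overlaps its Box trigger.
; The overlap increments Score1 on player 0's BP_MyPlayerState, then spawns the NS_Pickup effect and a sound at the actor's location.
; It also restarts the Z_Offset timeline, which animates the relative location of the 共産ブロック component.
; Despite the asset's name, the graph has no guard against repeat triggering.
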(event OnComponentBeginOverlap(Box)
  (params (OverlappedComponent :type Primitive%20Component%20Object%20Reference) (OtherActor :type Actor%20Object%20Reference) (OtherComp :type Primitive%20Component%20Object%20Reference) (OtherBodyIndex :type Integer) (bFromSweep :type Boolean) (SweepResult :type Hit%20Result%20Structure%20%28by%20ref%29))
  (bind _returnvalue (Transformation|GetActorLocation))
  (Utilities|Casting|CastToBP_ThirdPersonCharacter OtherActor)
  (bind _asbp_my_player_state (Utilities|Casting|CastToBP_MyPlayerState (Game|GetPlayerState 0)))
  (Math|Integer|IncrementInt (Variables|/Game/My_Game/Blueprint/BP_MyPlayerState.BP_MyPlayerState_C|GetScore1 _asbp_my_player_state)
    (:%20%20
      (Niagara|SpawnSystematLocation "/Game/My_Game/Effect/NS_Pickup.NS_Pickup" _returnvalue)
      (Audio|PlaySoundatLocation 0 _returnvalue "0, 0, 0" 1.0 1.0 0.0 0 0 0 0)
      (bind _新規track_0 (Timeline|Z_Offset PlayFromStart)
        (:Update
          (Transformation|SetRelativeLocation (Variables|Default|Get共産ブロック) (Math|Conversions|ToVector(Float) _新規track_0) false false))))))

(event EventBeginPlay)

(event Collision|EventActorBeginOverlap
  (params (OtherActor :type Actor%20Object%20Reference)))

(event EventTick
  (params (DeltaSeconds :type Float%20%28single-precision%29)))

(fn ConstructionScript)