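; BP_Enemy is a stationary-style enemy that tracks the player and fires a beam effect when something enters its detection sphere.
; Tick turns the actor toward the player's pitch and yaw using a look-at rotation.
; Sphere begin overlap plays an open animation, waits briefly, then spawns Niagara beam and effect systems aimed at the player; end overlap plays the close animation.
; The overlap is unfiltered and the beam is visual only, with no damage logic.
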(event OnComponentBeginOverlap(Sphere)
  (params (OverlappedComponent :type Primitive%20Component%20Object%20Reference) (OtherActor :type Actor%20Object%20Reference) (OtherComp :type Primitive%20Component%20Object%20Reference) (OtherBodyIndex :type Integer) (bFromSweep :type Boolean) (SweepResult :type Hit%20Result%20Structure%20%28by%20ref%29))
  (bind _returnvalue (Game|GetPlayerCharacter 0))
  (bind _returnvalue_2 (Transformation|GetActorLocation))
  (bind _returnvalue_3 (Transformation|GetActorLocation _returnvalue))
  (bind _returnvalue_4 (Math|Rotator|FindLookatRotation _returnvalue_2 _returnvalue_3))
  (bind (_roll _pitch _yaw) (Math|Rotator|BreakRotator _returnvalue_4))
  (Components|Animation|PlayAnimation (Variables|Default|GetSkeletalMesh) "/Game/My_Game/Object/Beam/Open_Anim.Open_Anim" false)
  (Utilities|FlowControl|Delay 1.8)
  (Niagara|SpawnSystematLocation "/Game/My_Game/Effect/NS_Beam.NS_Beam" _returnvalue_2 (Math|Rotator|MakeRotator 0.0 _pitch _yaw))
  (Niagara|SpawnSystematLocation "/Game/My_Game/Effect/NS_BeamEF.NS_BeamEF" _returnvalue_2))

(event OnComponentEndOverlap(Sphere)
  (params (OverlappedComponent :type Primitive%20Component%20Object%20Reference) (OtherActor :type Actor%20Object%20Reference) (OtherComp :type Primitive%20Component%20Object%20Reference) (OtherBodyIndex :type Integer))
  (Components|Animation|PlayAnimation (Variables|Default|GetSkeletalMesh) "/Game/My_Game/Object/Beam/Close_Anim.Close_Anim" false))

(event EventBeginPlay)

(event Collision|EventActorBeginOverlap
  (params (OtherActor :type Actor%20Object%20Reference)))

(event EventTick
  (params (DeltaSeconds :type Float%20%28single-precision%29))
  (bind _returnvalue (Game|GetPlayerCharacter 0))
  (bind _returnvalue_2 (Transformation|GetActorLocation))
  (bind _returnvalue_3 (Transformation|GetActorLocation _returnvalue))
  (bind _returnvalue_4 (Math|Rotator|FindLookatRotation _returnvalue_2 _returnvalue_3))
  (bind (_roll _pitch _yaw) (Math|Rotator|BreakRotator _returnvalue_4))
  (Transformation|SetActorRotation (Math|Rotator|MakeRotator 0.0 _pitch _yaw)))

(fn ConstructionScript)